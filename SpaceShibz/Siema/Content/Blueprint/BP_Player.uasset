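; Player actor that moves on the Y-Z plane from the MoveUp and MoveRight axis inputs.
; BeginPlay caches BP_GameMode, then a timeline lifts the player while spinning it, setting MoveEnabled when finished.
; The Movement function eases each axis speed toward its input target with FInterpTo.
; Tick applies both speeds as a swept per-frame offset and turns the yaw in proportion to horizontal speed.
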(event EventBeginPlay
  ;[1 1 1] Player
  (bind _asbp_game_mode (Utilities|Casting|CastToBP_GameMode (Game|GetGameMode)))
  (Variables|Default|SetBP_GameMode _asbp_game_mode)
  (Variables|Default|SetYaw (.Yaw (Math|Rotator|BreakRotator (Transformation|GetActorRotation))))
  (Variables|Default|SetSpawnLocation (Transformation|GetActorLocation))
  (bind _speed (Timeline|SpawnAnimation Play)
    (:Update
      (Transformation|SetActorLocationAndRotation (Math|Vector|Lerp(Vector) (Variables|Default|GetSpawnLocation) (+ (Variables|Default|GetSpawnLocation) "0, 0,60.000000") _speed) "0, 0, 0")
      (Transformation|SetActorRotation (Math|Rotator|Lerp(Rotator) "0, 0, 0" (Math|Rotator|MakeRotator 0.0 0.0 (+ (Variables|Default|GetYaw) 1.44e+03)) _speed)))
    (:Finished
      (Variables|Default|SetMoveEnabled true))))

(event Collision|EventActorBeginOverlap
  (params (OtherActor :type Actor%20Object%20Reference)))

(event EventTick
  (params (DeltaSeconds :type Float%20%28single-precision%29))
  ;[1 1 1] Movement
  (Variables|Default|SetDeltaSeconds DeltaSeconds)
  (Transformation|SetActorLocation (+ (Transformation|GetActorLocation) (Math|Vector|MakeVector 0.0 (Variables|Default|GetHozSpeed) (Variables|Default|GetVertSpeed))) true false)
  (Transformation|SetActorRotation (Class|KismetMathLibrary|RInterptoConstant (Transformation|GetActorRotation) (Math|Rotator|MakeRotator 0.0 0.0 (+ (* (Variables|Default|GetHozSpeed) 3.0) (Variables|Default|GetYaw))) (Variables|Default|GetDeltaSeconds) 6e+01)))

(event Input|AxisEvents|InputAxisMoveUp
  (params (AxisValue :type Float%20%28single-precision%29))
  ;[1 1 1] Movement
  (bind _returndirectionspeed (CallFunction|Movement (Variables|Default|GetVertSpeed) AxisValue))
  (Variables|Default|SetVertSpeed _returndirectionspeed))

(event Input|AxisEvents|InputAxisMoveRight
  (params (AxisValue :type Float%20%28single-precision%29))
  ;[1 1 1] Movement
  (bind _returndirectionspeed (CallFunction|Movement (Variables|Default|GetHozSpeed) AxisValue))
  (Variables|Default|SetHozSpeed _returndirectionspeed))

(fn ConstructionScript)

(fn Movement
  (params (Speed :type Float%20%28single-precision%29) (Direction :type Float%20%28single-precision%29))
  (return (Math|Interpolation|FInterpTo Speed (* (Variables|Default|GetMovementSpeed) Direction) (Variables|Default|GetDeltaSeconds) 6.0)))