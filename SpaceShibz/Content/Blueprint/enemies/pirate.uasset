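; Pirate enemy actor that wanders side to side along Y while facing the player.
; SetNewTargetLocation takes the player pawn's X and Z with a random Y as the target, on BeginPlay and again on each arrival.
; While MoveAvailable is set, Tick moves the actor there at constant speed without sweep and turns it toward the player.
; Debug prints remain on target selection and arrival.
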(event Custom|SetNewTargetLocation
  (bind _asbp_player (Utilities|Casting|CastToBP_Player (Game|Player|GetPlayerPawn 0)))
  (bind _output_get (Variables|Default|SetHeight (.x (Transformation|GetActorLocation _asbp_player))))
  (bind _output_get_2 (Variables|Default|SetcurrZ (.z (Transformation|GetActorLocation _asbp_player))))
  (bind _output_get_3 (Variables|Default|SetcurrY (Math|Random|RandomFloatinRange -8e+02 7.6e+02)))
  (bind _output_get_4 (Variables|Default|SetTarget (Math|Vector|MakeVector _output_get _output_get_3 _output_get_2)))
  (Development|PrintString (Utilities|String|ToString(Vector) _output_get_4))
  (Development|PrintString (Utilities|String|ToString(Vector) (Transformation|GetActorLocation))))

(event EventBeginPlay
  (Utilities|Casting|CastToBP_Player (Game|Player|GetPlayerPawn 0))
  (CallFunction|SetNewTargetLocation))

(event Collision|EventActorBeginOverlap
  (params (OtherActor :type Actor%20Object%20Reference)))

(event EventTick
  (params (DeltaSeconds :type Float%20%28single-precision%29))
  (if (Variables|Default|GetMoveAvailable)
    (Transformation|SetActorLocation (Math|Interpolation|VInterptoConstant (Transformation|GetActorLocation) (Variables|Default|GetTarget) (Utilities|Time|GetWorldDeltaSeconds) 5e+02) false false)
    (Transformation|SetActorRotation (Math|Rotator|FindLookatRotation (Transformation|GetActorLocation) (Transformation|GetActorLocation (Game|Player|GetPlayerPawn 0))))
    (if (Math|Vector|Equal(Vector) (Transformation|GetActorLocation) (Variables|Default|GetTarget) 0.1)
      (Variables|Default|SetMoveAvailable true)
      (Development|PrintString "Hello")
      (CallFunction|SetNewTargetLocation))))

(fn ConstructionScript)