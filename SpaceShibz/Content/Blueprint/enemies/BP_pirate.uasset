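; Pirate enemy that moves on the player's X plane, hopping between random Y targets while stepping down in height, and fires missiles on a timer.
; Tick drives constant-speed movement, shooting and HpCheck, which applies queued damage and reveals fire effects at low health.
; Death plays an explosion, notifies BP_Player, spawns a BP_point and destroys the actor.
; Level scales maximum missile damage; the face-player rotation is unconnected.
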(event Custom|SetNewTargetLocation
  ;[1 1 1] Ustawia nowy punkt do którego pirat będzie dążyć
  (if (Variables|Default|GetisAlive)
    (if (> (Variables|Default|GetcurrZ) 2e+02)
      (bind _output_get (Variables|Default|SetcurrZ (- (Variables|Default|GetcurrZ) (Math|Random|RandomFloatinRange 15.0 3e+01)))))
    (bind _output_get_2 (Variables|Default|SetcurrY (Math|Random|RandomFloatinRange -8e+02 7.6e+02)))
    (Variables|Default|SetTarget (Math|Vector|MakeVector (Variables|Default|GetDepth) _output_get_2 _output_get))))

(event Custom|Shoot
  ;[1 1 1] Poruszanie się i strzelanie
  ;;[1 1 1] Shoot
  (Game|SpawnActorfromClass "/Game/Blueprint/missiles/BP_Missile1.BP_Missile1_C" (Math|Transform|MakeTransform (Transformation|GetWorldLocation (Variables|Default|GetShoot_Pos)) (.rotation (Transformation|GetWorldTransform (Variables|Default|GetShoot_Pos)))) "AlwaysSpawn" 0 (Math|Random|RandomFloatinRange (Variables|Default|GetminDmg) (Variables|Default|GetmaxDmg)) (Variables|Default|GetShoot%20Speed) false 0))

(event Custom|Hp%20Check
  (params (HP :type Float%20%28single-precision%29))
  (bind _maxhp (Variables|Default|GetmaxHP))
  (bind _returnvalue (/ HP _maxhp))
  ;[1 1 1] sprawdzanie czy żyje i ogarnia sytuacje jeżeli nie żyje
  (Variables|Default|SetHP (- (Variables|Default|GetHP) (Variables|Default|GetDamage%20To%20Calculate)))
  (Variables|Default|SetDamage%20To%20Calculate 0.0)
  (if (<= HP 0.0) ; Czy nieżyje
    (Variables|Default|SetminTimeBetweenShoots 1e+01)
    (Components|Activation|SetActive (Variables|Default|GetExplosion) true false)
    (Rendering|SetVisibility (Variables|Default|GetPirate%20Model) false true)
    (bind _asbp_player (Utilities|Casting|CastToBP_Player (Game|Player|GetPlayerPawn 0)))
    (Default|EnemyDestroyed _asbp_player "NewEnumerator0")
    (Variables|Default|SetisAlive false)
    (Components|Activation|SetActive (Variables|Default|GetFire_1) false false)
    (Utilities|FlowControl|Delay 0.5)
    (Components|Activation|SetActive (Variables|Default|GetExplosion) false false)
    (Game|SpawnActorfromClass "/Game/Blueprint/enemies/BP_point.BP_point_C" (Transformation|GetActorTransform) "AlwaysSpawn" 0 "NewEnumerator0" 0)
    (Components|Activation|SetActive (Variables|Default|GetFire_2) false false)
    (Utilities|FlowControl|Delay 0.5)
    (Actor|DestroyActor)
    (elif (<= _returnvalue 0.3)
      (Rendering|SetVisibility (Variables|Default|GetFire_1) true false)
      (if (<= _returnvalue 0.15)
        (Rendering|SetVisibility (Variables|Default|GetFire_2) true false)))))

(event EventBeginPlay
  ;[1 1 1] Ustaw się na poziomie gracza
  (bind _asbp_player (Utilities|Casting|CastToBP_Player (Game|Player|GetPlayerPawn 0)))
  (Variables|Default|SetcurrZ 6e+02)
  (Variables|Default|SetDepth (.x (Transformation|GetActorLocation _asbp_player)))
  (CallFunction|SetNewTargetLocation)
  (Transformation|SetActorLocation (Variables|Default|GetTarget) false true)
  (Variables|Default|SetmaxHP (Variables|Default|GetHP))
  (Variables|Default|SetMaxDmg (* (Variables|Default|GetMinDmg) (Math|Conversions|ToFloat(Integer) (Variables|Default|Getlevel)))))

(event Collision|EventActorBeginOverlap
  (params (OtherActor :type Actor%20Object%20Reference)))

(event EventTick
  (params (DeltaSeconds :type Float%20%28single-precision%29))
  ;[1 1 1] Poruszanie się i strzelanie
  (if (Variables|Default|GetisAlive)
    (bind _output_get (Variables|Default|SetTime%20from%20last%20shot (+ DeltaSeconds (Variables|Default|GetTime%20from%20last%20shot))))
    (CallFunction|HpCheck (Variables|Default|GetHP))
    (if (> _output_get (Variables|Default|GetminTimeBetweenShoots))
      (CallFunction|Shoot)
      (Variables|Default|SetTime%20from%20last%20shot 0.0))
    (if (Variables|Default|GetMoveAvailable)
      (Transformation|SetActorLocation (Math|Interpolation|VInterptoConstant (Transformation|GetActorLocation) (Variables|Default|GetTarget) (Utilities|Time|GetWorldDeltaSeconds) (Variables|Default|GetInterp%20Speed)) false false)
      (if (Math|Vector|Equal(Vector) (Transformation|GetActorLocation) (Variables|Default|GetTarget) 0.001)
        (Variables|Default|SetMoveAvailable true)
        (CallFunction|SetNewTargetLocation)))))

(fn ConstructionScript)