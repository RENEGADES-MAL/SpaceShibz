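; BP_zoid is an enemy that spawns at a random horizontal position up high and descends at a random constant speed.
; Touching the player sets the player's pending damage to a random level-scaled amount and kills the zoid.
; Tick moves it and subtracts its pending damage from HP; death plays an explosion and spawns a BP_point before destruction.
; Both death and reaching the bottom notify BP_Player through EnemyDestroyed.
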(event Custom|Hp%20Check
  ;[1 1 1] Sprawdza czy zyje
  (Variables|Default|SetHP (- (Variables|Default|GetHP) (Variables|Default|GetDamage%20To%20Calculate)))
  (Variables|Default|SetDamage%20To%20Calculate 0.0)
  (if (<= (Variables|Default|GetHP) 0.0) ; Czy nieżyje
    (Components|Activation|SetActive (Variables|Default|GetZoidExplosion) true false)
    (Rendering|SetVisibility (Variables|Default|GetZoid%20Model) false true)
    (bind _asbp_player (Utilities|Casting|CastToBP_Player (Game|Player|GetPlayerPawn 0)))
    (Default|EnemyDestroyed _asbp_player "NewEnumerator1")
    (Variables|Default|SetisAlive false)
    (Utilities|FlowControl|Delay 0.5)
    (Components|Activation|SetActive (Variables|Default|GetZoidExplosion) false false)
    (Game|SpawnActorfromClass "/Game/Blueprint/enemies/BP_point.BP_point_C" (Transformation|GetActorTransform) "AlwaysSpawn" 0 "NewEnumerator0" 0)
    (Utilities|FlowControl|Delay 0.5)
    (Actor|DestroyActor)))

(event EventBeginPlay
  (bind _returnvalue (Transformation|GetActorLocation))
  (bind _output_get (Variables|Default|SetCurrY (Math|Random|RandomFloatinRange -8e+02 7.6e+02)))
  (bind _output_get_2 (Variables|Default|SetcurrZ 6e+02))
  (Variables|Default|SetDepth 0.0)
  (Transformation|SetActorLocation (Math|Vector|MakeVector 0.0 _output_get _output_get_2) false true)
  (Variables|Default|SetmaxHP (Variables|Default|GetHP))
  (Variables|Default|SetMaxDmg (* (Variables|Default|GetMinDmg) (Math|Conversions|ToFloat(Integer) (Variables|Default|Getlevel))))
  (Variables|Default|SetTarget (Math|Vector|MakeVector (.x _returnvalue) (.y _returnvalue) -5e+02))
  (Variables|Default|SetInterp%20Speed (Math|Random|RandomFloatinRange 2e+01 (Variables|Default|GetmaxSpeed))))

(event Collision|EventActorBeginOverlap
  (params (OtherActor :type Actor%20Object%20Reference))
  (bind _asbp_player (Utilities|Casting|CastToBP_Player OtherActor))
  (bind _output_value (CallFunction|AddDamage (Variables|/Game/Blueprint/BP_Player.BP_Player_C|GetDamage%20To%20Calculate _asbp_player)))
  (Variables|/Game/Blueprint/BP_Player.BP_Player_C|SetDamage%20To%20Calculate _asbp_player _output_value)
  (Variables|Default|SetHP 0.0))

(event EventTick
  (params (DeltaSeconds :type Float%20%28single-precision%29))
  (if (Variables|Default|GetisAlive)
    (Transformation|SetActorLocation (Math|Interpolation|VInterptoConstant (Transformation|GetActorLocation) (Variables|Default|GetTarget) (Utilities|Time|GetWorldDeltaSeconds) (Variables|Default|GetInterp%20Speed)) false false)
    (CallFunction|HpCheck)
    (if (Math|Vector|Equal(Vector) (Transformation|GetActorLocation) (Variables|Default|GetTarget) 0.001)
      (bind _asbp_player (Utilities|Casting|CastToBP_Player (Game|Player|GetPlayerPawn 0)))
      (Default|EnemyDestroyed _asbp_player "NewEnumerator1")
      (Actor|DestroyActor))))

(fn ConstructionScript)

(fn AddDamage
  (params (Input :type Float%20%28single-precision%29))
  (bind _mindmg (Variables|Default|GetMinDmg))
  (return (+ 0.0 (Math|Random|RandomFloatinRange _mindmg (* _mindmg (Math|Conversions|ToFloat(Integer) (Variables|Default|Getlevel)))))))