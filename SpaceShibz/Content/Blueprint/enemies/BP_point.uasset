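; BP_point is a collectible point pickup of a given PointType (Kosmoszafir or Kosmorubin) that awards points to the player.
; BeginPlay shows the mesh, though both types reveal the Kosmoszafir component.
; Tick spins it around yaw and moves it at constant speed toward world location (0, 0, -1000), destroying it on arrival.
; Overlap with BP_Player passes the type to AddPoints, plays a sound and destroys the pickup.
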(event EventBeginPlay
  (Variables|Default|SetTarget (Math|Vector|MakeVector 0.0 0.0 -1e+03))
  (switch Utilities|FlowControl|Switch|SwitchonPoints (Variables|Default|GetPoint%20Type)
    (:NewEnumerator0
      (Rendering|SetVisibility (Variables|Default|GetKosmoszafir) true false))
    (:NewEnumerator1
      (Rendering|SetVisibility (Variables|Default|GetKosmoszafir) true false))))

(event Collision|EventActorBeginOverlap
  (params (OtherActor :type Actor%20Object%20Reference))
  (bind _asbp_player (Utilities|Casting|CastToBP_Player OtherActor))
  (Default|AddPoints _asbp_player (Variables|Default|GetPoint%20Type))
  (Audio|PlaySound2D "/Game/Assets/Sounds/Points/Point_Cue.Point_Cue" 1.0 1.0 0.0 0 0)
  (Actor|DestroyActor))

(event EventTick
  (params (DeltaSeconds :type Float%20%28single-precision%29))
  (Transformation|SetActorLocation (Math|Interpolation|VInterptoConstant (Transformation|GetActorLocation) (Variables|Default|GetTarget) (Utilities|Time|GetWorldDeltaSeconds) (Variables|Default|GetInterp%20Speed)) false false)
  (Transformation|SetActorRotation (Class|KismetMathLibrary|RInterptoConstant (Transformation|GetActorRotation) (Math|Rotator|MakeRotator 0.0 0.0 (+ (.yaw (Transformation|GetActorRotation)) 3e+01)) DeltaSeconds 6e+01))
  (if (Math|Vector|Equal(Vector) (Transformation|GetActorLocation) (Variables|Default|GetTarget) 0.001)
    (Actor|DestroyActor)))

(fn ConstructionScript)