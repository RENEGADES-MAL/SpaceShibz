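; Rocket explosion actor that plays a hit effect and damages actors that overlap it.
; On BeginPlay, OnHitExplosion runs for EmittingTime, is deactivated, then the actor destroys itself after DelayAfterEmmiting.
; Each begin overlap sends DamageToDeal through AddDamageMessage to actors implementing the DamageControll interface.
; Overlap damage is not gated by the emission timer, so it can still occur until the actor is destroyed.
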(event EventBeginPlay
  (Utilities|FlowControl|Delay (Variables|Default|GetEmittingTime))
  (Components|Activation|SetActive (Variables|Default|GetonHitExplosion) false false)
  (Utilities|FlowControl|Delay (Variables|Default|GetDelayAfterEmmiting))
  (Actor|DestroyActor))

(event Collision|EventActorBeginOverlap
  (params (OtherActor :type Actor%20Object%20Reference))
  (if (Utilities|DoesObjectImplementInterface OtherActor "/Game/Blueprint/Interfaces_and_functions/DamageControll.DamageControll_C")
    (Class|DamageControll|AddDamage(Message) OtherActor (Variables|Default|GetDamageToDeal))))

(fn ConstructionScript)