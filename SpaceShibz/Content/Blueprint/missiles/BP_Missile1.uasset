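; Missile projectile, friendly or enemy by the FriendlyMissile flag, which picks its launch sound, travel direction and an orange material for enemies.
; Tick eases it along world Z with VInterpTo toward a fixed limit and destroys it on nearing that point.
; On overlap, DamageControll actors take damage via AddDamageMessage only across sides (enemy missiles hit BP_Player, friendly ones anything else), then an explosion spawns and the missile is destroyed.
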(event Custom|Handle%20HIt
  ;[1 1 1] Tworzy obiekt z particlesami trafienia i niszczy pocisk
  (Game|SpawnActorfromClass "/Game/Blueprint/missiles/onHitExplosion.onHitExplosion_C" (Transformation|GetActorTransform) "Undefined" 0 0.1 1.0 0)
  (Actor|DestroyActor))

(event EventBeginPlay
  (bind _friendlymissile (Variables|Default|GetFriendlyMissile))
  (Audio|PlaySound2D (select _friendlymissile "/Game/Assets/Sounds/Missiles/Friendly/Missile_Friendly_Cue.Missile_Friendly_Cue" "/Game/Assets/Sounds/Missiles/Non-Friendly/Missile_Enemy_Cue.Missile_Enemy_Cue") 1.0 1.0 0.0 0 0)
  (if (not _friendlymissile)
    (Rendering|Material|SetMaterial (Variables|Default|GetStaticMesh) 0 "/Game/Materials/M_ORANGE_EMISSIVE.M_ORANGE_EMISSIVE")))

(event Collision|EventActorBeginOverlap
  (params (OtherActor :type Actor%20Object%20Reference))
  (bind _friendlymissile (Variables|Default|GetFriendlyMissile))
  ;[1 1 1] Ogarnia trafienia
  (if (Utilities|DoesObjectImplementInterface OtherActor "/Game/Blueprint/Interfaces_and_functions/DamageControll.DamageControll_C")
    (Utilities|Casting|CastToBP_Player OtherActor
      (:then
        (if (not _friendlymissile)
          (Class|DamageControll|AddDamage(Message) OtherActor (Variables|Default|GetDmg) :!label _label)
          (CallFunction|HandleHIt)))
      (:CastFailed
        (if _friendlymissile
          (goto _label))))))

(event EventTick
  (params (DeltaSeconds :type Float%20%28single-precision%29))
  (bind _returnvalue (Transformation|GetActorLocation))
  (bind _friendlymissile (Variables|Default|GetFriendlyMissile))
  (bind _returnvalue_2 (Math|Float|SelectFloat 2e+03 -2e+03 _friendlymissile))
  (bind _returnvalue_3 (Math|Vector|MakeVector (.x _returnvalue) (.y _returnvalue) _returnvalue_2))
  (Transformation|SetActorLocation (Math|Interpolation|VInterpTo (Transformation|GetActorLocation) _returnvalue_3 DeltaSeconds (* (Variables|Default|GetSpeed) 0.75)) false false)
  (if (Math|Vector|Equal(Vector) _returnvalue_3 (Transformation|GetActorLocation) 1e+02)
    (Actor|DestroyActor)))

(fn ConstructionScript)