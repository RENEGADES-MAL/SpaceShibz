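; BP_Missile1_FRIENDLY is a friendly missile that damages pirates on contact.
; Each tick it moves along Z toward a fixed height at constant Speed, keeping its X and Y, and destroys itself on arrival.
; Overlapping a BP_pirate subtracts Dmg directly from that pirate's HP and destroys the missile; other actors are ignored.
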(event Custom|Handle%20Autodestroy
  (Actor|DestroyActor))

(event Collision|EventActorBeginOverlap
  (params (OtherActor :type Actor%20Object%20Reference))
  (bind _asbp_pirate (Utilities|Casting|CastToBP_pirate OtherActor))
  (Variables|/Game/Blueprint/enemies/BP_pirate.BP_pirate_C|SetHP _asbp_pirate (- (Variables|/Game/Blueprint/enemies/BP_pirate.BP_pirate_C|GetHP _asbp_pirate) (Variables|Default|GetDmg)))
  (CallFunction|HandleAutodestroy))

(event EventTick
  (params (DeltaSeconds :type Float%20%28single-precision%29))
  (bind _returnvalue (Transformation|GetActorLocation))
  (bind _output_get (Variables|Default|SetTarget (Math|Vector|MakeVector (.x _returnvalue) (.y _returnvalue) 6.5e+02)))
  (Transformation|SetActorLocation (Math|Interpolation|VInterptoConstant (Math|Vector|MakeVector (.x _returnvalue) (.y _returnvalue) (.z _returnvalue)) _output_get (Utilities|Time|GetWorldDeltaSeconds) (Variables|Default|GetSpeed)) false false)
  (if (Math|Vector|Equal(Vector) (Transformation|GetActorLocation) (Variables|Default|GetTarget) 0.1)
    (Actor|DestroyActor)))

(fn ConstructionScript)