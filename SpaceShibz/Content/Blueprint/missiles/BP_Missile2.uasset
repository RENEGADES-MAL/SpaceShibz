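; BP_Missile2 is a homing missile that seeks a random pirate, or a random drone when no pirates exist.
; Each tick it interpolates toward its target with compounding speed, retargeting if that becomes invalid and exploding if none remain.
; Overlapping a non-player actor that implements DamageControll sends damage, then spawns an explosion carrying half that damage and destroys the missile.
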(event Custom|GetNewTarget
  (bind _outactors (Actor|GetAllActorsOfClass "/Game/Blueprint/enemies/BP_pirate.BP_pirate_C"))
  (if (== (Utilities|Array|Length _outactors) 0)
    (bind _outactors_2 (Actor|GetAllActorsOfClass "/Game/Blueprint/enemies/BP_drone.BP_drone_C"))
    (if (== (Utilities|Array|Length _outactors_2) 0)
      (Development|PrintString "O kurde, nie mam co ze sobą zrobić. niszczę sie")
      (CallFunction|GenerateExplosion)
      (else
        (Variables|Default|SetTarget (Utilities|Array|Get(acopy) _outactors_2 (Math|Random|RandomInteger (Utilities|Array|Length _outactors_2))))))
    (else
      (Variables|Default|SetTarget (Utilities|Array|Get(acopy) _outactors (Math|Random|RandomInteger (Utilities|Array|Length _outactors)))))))

(event Custom|Destroy
  (Actor|DestroyActor))

(event Custom|GenerateExplosion
  (Game|SpawnActorfromClass "/Game/Blueprint/missiles/rocketExplosion.rocketExplosion_C" (Transformation|GetActorTransform) "AlwaysSpawn" 0 0.1 1.0 (* (Variables|Default|GetDmg) 0.5) 0)
  (Actor|DestroyActor))

(event Collision|EventActorBeginOverlap
  (params (OtherActor :type Actor%20Object%20Reference))
  (Utilities|Casting|CastToBP_Player OtherActor
    (:CastFailed
      (if (Utilities|DoesObjectImplementInterface OtherActor "/Game/Blueprint/Interfaces_and_functions/DamageControll.DamageControll_C")
        (Class|DamageControll|AddDamage(Message) OtherActor (Variables|Default|GetDmg))
        (CallFunction|GenerateExplosion)))))

(event EventTick
  (params (DeltaSeconds :type Float%20%28single-precision%29))
  (Variables|Default|SetActualMultiplier (+ (* DeltaSeconds (Variables|Default|GetSpeedMultiplier)) (Variables|Default|GetActualMultiplier)))
  (Variables|Default|GetTarget
    (:then
      (Transformation|SetActorLocation (Math|Interpolation|VInterptoConstant (Transformation|GetActorLocation) (Transformation|GetActorLocation (Variables|Default|GetTarget)) (Utilities|Time|GetWorldDeltaSeconds) (Variables|Default|GetSpeed)) false false)
      (Variables|Default|SetSpeed (* (Variables|Default|GetActualMultiplier) (Variables|Default|GetSpeed))))
    (:else
      (CallFunction|GetNewTarget))))

(fn ConstructionScript)