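; BP_Missile1_NONFRIENDLY is a hostile missile that travels straight along the Z axis and damages the player on contact.
; Each tick it interpolates at constant speed toward a fixed Z height at its current X and Y, without sweeping, and destroys itself on arrival.
; Overlapping BP_Player writes a random value between MinDmg and MaxDmg into the player's DamageToCalculate, then destroys the missile.
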(event Collision|EventActorBeginOverlap
  (params (OtherActor :type Actor%20Object%20Reference))
  (bind _asbp_player (Utilities|Casting|CastToBP_Player OtherActor))
  (Variables|/Game/Blueprint/BP_Player.BP_Player_C|SetDamage%20To%20Calculate _asbp_player (Math|Random|RandomFloatinRange (Variables|Default|GetminDmg) (Variables|Default|GetmaxDmg)))
  (Actor|DestroyActor))

(event EventTick
  (params (DeltaSeconds :type Float%20%28single-precision%29))
  (bind _returnvalue (Transformation|GetActorLocation))
  (bind _output_get (Variables|Default|SetTarget (Math|Vector|MakeVector (.x _returnvalue) (.y _returnvalue) -6.5e+02)))
  (Transformation|SetActorLocation (Math|Interpolation|VInterptoConstant (Math|Vector|MakeVector (.x _returnvalue) (.y _returnvalue) (.z _returnvalue)) _output_get (Utilities|Time|GetWorldDeltaSeconds) 7.5e+02) false false)
  (if (Math|Vector|Equal(Vector) (Transformation|GetActorLocation) (Variables|Default|GetTarget) 0.1)
    (Actor|DestroyActor)))

(fn ConstructionScript)