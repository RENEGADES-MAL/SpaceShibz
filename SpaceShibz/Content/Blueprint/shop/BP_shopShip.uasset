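; Shop ship actor that weaves across the player's depth plane, stepping gradually lower until it nears a floor height.
; BeginPlay snaps it to a first target with a brief spawn effect; Tick moves it at constant speed, picking a random sideways target on each arrival.
; If the player is dead, new targets drop far below.
; At zero HP it rises to an exit height, then destroys itself.
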(event Custom|SetNewTargetLocation
  ;[1 1 1] Ustawia nowy punkt do którego pirat będzie dążyć
  (if (Variables|Default|GetisAlive)
    (if (> (Variables|Default|GetcurrZ) 2e+02)
      (bind _output_get (Variables|Default|SetcurrZ (- (Variables|Default|GetcurrZ) (Math|Random|RandomFloatinRange 15.0 3e+01)))))
    (bind _output_get_2 (Variables|Default|SetcurrY (Math|Random|RandomFloatinRange -2e+02 2e+02)))
    (bind _asbp_player (Utilities|Casting|CastToBP_Player (Game|Player|GetPlayerPawn 0)))
    (Variables|Default|SetTarget (Math|Vector|MakeVector (Variables|Default|GetDepth) _output_get_2 (Math|Float|SelectFloat _output_get -1e+03 (Variables|/Game/Blueprint/BP_Player.BP_Player_C|GetIs%20Alive _asbp_player))))))

(event EventBeginPlay
  (bind _spawneffect (Variables|Default|GetSpawnEffect))
  ;[1 1 1] Ustaw się na poziomie gracza
  (bind _asbp_player (Utilities|Casting|CastToBP_Player (Game|Player|GetPlayerPawn 0)))
  (Variables|Default|SetcurrZ 9.2e+02)
  (Variables|Default|SetDepth (.x (Transformation|GetActorLocation _asbp_player)))
  (CallFunction|SetNewTargetLocation)
  (Transformation|SetActorLocation (Variables|Default|GetTarget) false true)
  (Variables|Default|SetmaxHP (Variables|Default|GetHP))
  (Components|Activation|SetActive _spawneffect true false)
  (Utilities|FlowControl|Delay 0.5)
  (Components|Activation|SetActive _spawneffect false false))

(event Collision|EventActorBeginOverlap
  (params (OtherActor :type Actor%20Object%20Reference)))

(event EventTick
  (params (DeltaSeconds :type Float%20%28single-precision%29))
  ;[1 1 1] Poruszanie się i strzelanie
  (if (Variables|Default|GetisAlive)
    ;[1 1 1] sprawdzanie czy żyje i ogarnia sytuacje jeżeli nie żyje
    (if (<= (Variables|Default|GetHP) 0.0) ; Czy nieżyje
      (Variables|Default|SetisAlive false)
      (Variables|Default|SetTarget (Math|Vector|MakeVector (.x (Variables|Default|GetTarget)) (.y (Variables|Default|GetTarget)) 1.1e+03))
      (Variables|Default|SetInterp%20Speed 4e+02)
      (elif (Variables|Default|GetMoveAvailable)
        (Transformation|SetActorLocation (Math|Interpolation|VInterptoConstant (Transformation|GetActorLocation) (Variables|Default|GetTarget) (Utilities|Time|GetWorldDeltaSeconds) (Variables|Default|GetInterp%20Speed)) false false)
        (if (Math|Vector|Equal(Vector) (Transformation|GetActorLocation) (Variables|Default|GetTarget) 0.001)
          (Variables|Default|SetMoveAvailable true)
          (CallFunction|SetNewTargetLocation))))
    (else
      (Transformation|SetActorLocation (Math|Interpolation|VInterptoConstant (Transformation|GetActorLocation) (Variables|Default|GetTarget) (Utilities|Time|GetWorldDeltaSeconds) (Variables|Default|GetInterp%20Speed)) false false)
      (if (Math|Vector|Equal(Vector) (Transformation|GetActorLocation) (Variables|Default|GetTarget) 0.001)
        (Actor|DestroyActor)))))

(fn ConstructionScript)