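; Shake utility whose ShakeIt function jitters three by-reference values by random amounts within plus or minus ShakeDrift.
; Each pass passes every value and its random offset through an unnamed helper, then writes the result back.
; The loop is a hand-wired branch with no delay, running while NumberOfShakes is below the incrementing ShakeCounter.
; As written, that comparison never turns false once entered, so the loop has no normal exit.
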(fn ShakeIt
  (params (Number%20Of%20Shakes :type Integer) (ShakeDrift :type Float%20%28single-precision%29) (Shake%20ref%201 :type Float%20%28single-precision%29%20%28by%20ref%29) (Shake%20ref%202 :type Float%20%28single-precision%29%20%28by%20ref%29) (Shake%20ref%203 :type Float%20%28single-precision%29%20%28by%20ref%29))
  (bind _returnvalue (* -1.0 ShakeDrift))
  (bind _shakecounter (LocalVariables|GetShakeCounter))
  (bind _returnvalue_2 (Math|Random|RandomFloatinRange _returnvalue ShakeDrift))
  (if (< Number%20Of%20Shakes _shakecounter) :!label _label ; Start Loopa
    (Math|Integer|IncrementInt _shakecounter
      (:%20%20
        (bind _changed_value (CallFunction|+= Shake%20ref%201 _returnvalue_2))
        (|SetBy-RefVar Shake%20ref%201 _changed_value)
        (bind _changed_value_2 (CallFunction|+= Shake%20ref%202 _returnvalue_2))
        (|SetBy-RefVar Shake%20ref%202 _changed_value_2)
        (bind _changed_value_3 (CallFunction|+= Shake%20ref%203 _returnvalue_2))
        (|SetBy-RefVar Shake%20ref%203 _changed_value_3)
        (goto _label)))))