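; Player spaceship for a shooter, which also runs enemy wave spawning, kill and point counting, and opens the upgrade shop once a wave is cleared.
; Tick drives upgrade-scaled auto-fire, interpolated movement with yaw turning, and bounds checks that reverse and damp outward velocity.
; Damage drains a regenerating shield before health, which controls fire effects, death explosion and UI notification.
; E launches a second missile type when pirates exist.
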(event Custom|Check%20HP%20level
  (bind _fire_1 (Variables|Default|GetFire_1))
  (bind _health (Variables|HP|GetHealth))
  (bind _maxhealth (Variables|HP|GetMaxHealth))
  (bind _returnvalue (/ _health _maxhealth))
  ;[1 1 1] Wszystkie rzeczy związane z ogniem i eksplozjami
  (if (<= _health 0.0) ; Czy nieżyje
    (Variables|Missile1|SetMissile1%20Time%20Between%20Shoots 1e+01)
    (CallFunction|DissableUI)
    (Components|Activation|SetActive (Variables|Default|GetExplosion) true false)
    (Rendering|SetVisibility (Variables|Default|GetPlayerMesh) false true)
    (Variables|Default|SetIs%20Alive false)
    (Components|Activation|SetActive (Variables|Default|GetFire_1) false false)
    (Utilities|FlowControl|Delay 0.5)
    (Components|Activation|SetActive (Variables|Default|GetExplosion) false false)
    (Components|Activation|SetActive (Variables|Default|GetFire_2) false false)
    (Utilities|FlowControl|Delay 0.5)
    (Actor|DestroyActor)
    (elif (<= _returnvalue 0.3)
      (Components|Activation|SetActive _fire_1 true false)
      (if (<= _returnvalue 0.15)
        (Components|Activation|SetActive (Variables|Default|GetFire_2) true false))
      (else
        (Components|Activation|SetActive _fire_1 false false)
        (Components|Activation|SetActive (Variables|Default|GetFire_2) false false)))))

(event Custom|Spawn%20Shop
  ;[1 1 1] Uruchamia sklep
  (Variables|Default|SetShop%20is%20on%20screen true)
  (bind _returnvalue (UserInterface|CreateWidget "/Game/Blueprint/shop/shopMenu.shopMenu_C" 0 (Variables|HP|GetHp%20cost) (Variables|HP|GetHp%20per%20Heal) (Variables|Missile1|GetMissile1%20upgrade%20level) (Variables|Missile1|GetMissile1%20upgrade%20cost) (Variables|Missile2|GetMissile2%20upgrade%20level) (Variables|Missile2|GetMissile2%20upgrade%20cost) (Variables|HP|GetArmor%20Level) (Variables|HP|GetArmor%20upgrade%20cost) (Variables|HP|GetHP%20per%20upgrade) (Variables|Mobility|GetMobility%20level) (Variables|Mobility|GetMobility%20upgrade%20cost)))
  (UserInterface|Viewport|AddtoViewport _returnvalue 0)
  (Variables|Shield|SetShield (Variables|Shield|GetMaxShield)))

(event Custom|Handle%20Enemy%20spawn
  (bind _returnvalue (Transformation|GetActorTransform))
  (bind _max_enemies_level (Variables|enemies|Getmax%20Enemies%20level))
  (bind _returnvalue_2 (Math|Random|RandomIntegerinRange 1 _max_enemies_level))
  ;[1 1 1] Ogarnia respienie wrogów
  (bind _output_get (Variables|enemies|SetTime%20From%20Last%20Enemy%20Spawned (+ (Variables|enemies|GetTime%20From%20Last%20Enemy%20Spawned) (Variables|Default|GetDeltaSeconds))))
  (if (Math|Boolean|ANDBoolean (> _output_get (Variables|enemies|GetTime%20Between%20Spawns)) (< (Variables|enemies|GetLiving%20Enemies) (Variables|enemies|Getmax%20enemies%20on%20screen)) (> (Variables|enemies|GetEnemies%20To%20Spawn) 0))
    (Variables|enemies|SetTime%20From%20Last%20Enemy%20Spawned 0.0)
    (switch int (Variables|enemies|GetEnemies%20To%20Spawn)
      (:Default
        (switch int (Math|Random|RandomIntegerinRange 1 2)
          (:1
            (Game|SpawnActorfromClass "/Game/Blueprint/enemies/BP_pirate.BP_pirate_C" (Math|Transform|MakeTransform (.location _returnvalue) "0, 0, 0" (.scale _returnvalue)) "Undefined" 0 5e+02 1.0 1e+02 _returnvalue_2 0 :!label _label)
            (Development|PrintString "Respie pirata"))
          (:2
            (Game|SpawnActorfromClass "/Game/Blueprint/enemies/BP_zoid.BP_zoid_C" (Math|Transform|MakeTransform (.location (Transformation|GetActorTransform)) "0, 0, 0" "1,1,1") "AlwaysSpawn" 0 4e+02 2e+01 _returnvalue_2 0)
            (Development|PrintString "Respie Zoida" true true "(R=0.000000,G=0.660000,B=1.000000,A=1.000000)" 5.0))))
      (:1
        (goto _label)))
    (bind _result (Math|Integer|IncrementInt (Variables|enemies|GetLiving%20Enemies))
      (:%20%20
        (Development|PrintString (Utilities|String|Append "Dodaje żyjącego przeciwnika. obecnie: " (Utilities|String|ToString(Integer) _result)))
        (bind _result_2 (Math|Integer|DecrementInt (Variables|enemies|GetEnemies%20To%20Spawn))
          (:%20%20
            (Development|PrintString (Utilities|String|Append "Odejmuje wroga do zrespienia, obecnie: " (Utilities|String|ToString(Integer) _result_2)))))))))

(event Custom|Handle%20Shoot%20Request
  ;[1 1 1] Autostrzelanie
  (if (not (Variables|Default|GetShop%20is%20on%20screen))
    (if (>= (Variables|Missile1|GetMIssile1%20Time%20From%20Last%20Shoot) (Variables|Missile1|GetMissile1%20Time%20Between%20Shoots))
      (Game|SpawnActorfromClass "/Game/Blueprint/missiles/BP_Missile1.BP_Missile1_C" (Math|Transform|MakeTransform (Transformation|GetWorldLocation (Variables|Default|GetShoot_Pos))) "AlwaysSpawn" 0 (+ (* (Variables|Missile1|GetMissile1%20damage%20per%20upgrade) (Math|Conversions|ToFloat(Integer) (Variables|Missile1|GetMissile1%20upgrade%20level))) (Variables|Missile1|GetMissile1%20base%20damage)) (+ (Variables|Missile1|GetMissile1%20base%20speed) (* (Math|Conversions|ToFloat(Integer) (Variables|Missile1|GetMissile1%20upgrade%20level)) (Variables|Missile1|GetMissile1%20speed%20per%20upgrade))) true 0)
      (Variables|Missile1|SetMIssile1%20Time%20From%20Last%20Shoot (- (stale _output_get) (Variables|Missile1|GetMissile1%20Time%20Between%20Shoots)))
      (else
        (bind _output_get (Variables|Missile1|SetMIssile1%20Time%20From%20Last%20Shoot (+ (Variables|Missile1|GetMIssile1%20Time%20From%20Last%20Shoot) (Variables|Default|GetDeltaSeconds))))))))

(event Custom|Handle%20Shield%20Renew
  (params (Delta%20Seconds :type Float%20%28single-precision%29))
  (bind _maxshield (Variables|Shield|GetMaxShield))
  ;[1 1 1] Handle Shield Renew
  (Variables|Shield|SetTime%20From%20Last%20Shield%20Renew (+ (Variables|Shield|GetTime%20From%20Last%20Shield%20Renew) Delta%20Seconds))
  (bind _output_get (Variables|Shield|SetTime%20From%20Last%20Damage (+ Delta%20Seconds (Variables|Shield|GetTime%20From%20Last%20Damage))))
  (if (and (> _output_get (Variables|Shield|GetTime%20Required%20To%20Start%20Renewing%20Shield)) (< (Variables|Shield|GetShield) (Variables|Shield|GetMaxShield))) ; Jeżeli można odnawiać tarcze
    (if (<= (Variables|Shield|GetShield) 0.0)
      (Audio|PlaySound2D "/Game/Assets/Sounds/Shield/Shield_up_Cue.Shield_up_Cue" 1.0 1.0 0.0 0 0))
    (if (>= (Variables|Shield|GetTime%20From%20Last%20Shield%20Renew) 1.0) ; Jeżeli czas od ostatniego odnowienia jest większy/równy 1
      (Variables|Shield|SetTime%20From%20Last%20Shield%20Renew 0.0)
      (if (>= (/ (Variables|Shield|GetShield) _maxshield) 0.5) ; Jeżeli tarcza jest równa/większa połowie
        (Variables|Shield|SetShield (+ (Variables|Shield|GetShield) (* (Variables|Shield|GetMaxShield) 0.1)))
        (else
          (Variables|Shield|SetShield (+ (Variables|Shield|GetShield) (* _maxshield 0.05))))))))

(event Custom|Dissable%20UI
  ;[1 1 1] Wyłącza standardowe UI i informuje UI o przegranej
  (bind _asmain_ui (Utilities|Casting|CastTomainUI (Variables|Default|GetcurrUI)))
  (Variables|/Game/Blueprint/mainUI.mainUI_C|SetPlayerIsAlive _asmain_ui false))

(event Custom|enemy%20Destroyed
  (params (Enemy%20type :type Enemies%20Enum :default "NewEnumerator0"))
  ;[1 1 1] Liczy zabitych wrogów
  (Math|Integer|IncrementInt (Variables|Stats|GetDestroyed%20Enemies)
    (:%20%20
      (Math|Integer|DecrementInt (Variables|enemies|GetLiving%20Enemies)
        (:%20%20
          (switch Utilities|FlowControl|Switch|SwitchonEnemies Enemy%20type
            (:NewEnumerator0
              (Math|Integer|IncrementInt (Variables|Stats|GetDestroyed%20Pirates)))
            (:NewEnumerator1
              (Math|Integer|IncrementInt (Variables|Stats|GetDestroyed%20Zoids)))))))))

(event Custom|Handle%20out%20of%20map%20exception%20%28Z%20axis%29
  ;[1 1 1] Odpowiada za skryptowe uniemożliwianie wylatywania za mape
  (Variables|Default|SetExceptionAxis "NewEnumerator1")
  (bind (_hoz_speed _vert_speed) (CallFunction|HandleOutOfMapException (Transformation|GetActorLocation) (Variables|Movement|GetHozSpeed) (Variables|Movement|GetVertSpeed) (Variables|Default|GetExceptionAxis)))
  (Variables|Movement|SetHozSpeed _hoz_speed)
  (Variables|Movement|SetVertSpeed _vert_speed))

(event Custom|Add%20points
  (params (NewParam :type Points%20Enum :default "NewEnumerator0"))
  ;[1 1 1] Odpowiada za dodawanie punktów
  (switch Utilities|FlowControl|Switch|SwitchonPoints NewParam
    (:NewEnumerator0
      (Variables|Default|SetPoints (+ (Variables|Default|GetPoints) 1)))
    (:NewEnumerator1
      (Variables|Default|SetPoints (+ (Variables|Default|GetPoints) 5)))))

(event Custom|Handle%20out%20of%20map%20exception%20%28Y%20axis%29
  ;[1 1 1] Odpowiada za skryptowe uniemożliwianie wylatywania za mape
  (Variables|Default|SetExceptionAxis "NewEnumerator0")
  (bind (_hoz_speed _vert_speed) (CallFunction|HandleOutOfMapException (Transformation|GetActorLocation) (Variables|Movement|GetHozSpeed) (Variables|Movement|GetVertSpeed) (Variables|Default|GetExceptionAxis)))
  (Variables|Movement|SetHozSpeed _hoz_speed)
  (Variables|Movement|SetVertSpeed _vert_speed))

(event EventBeginPlay
  ;[1 1 1] Player
  (bind _returnvalue (UserInterface|CreateWidget "/Game/Blueprint/mainUI.mainUI_C"))
  (Variables|Default|SetcurrUI _returnvalue)
  (UserInterface|Viewport|AddtoViewport _returnvalue 0)
  (bind _asbp_game_mode (Utilities|Casting|CastToBP_GameMode (Game|GetGameMode)))
  (Variables|Default|SetBP_GameMode _asbp_game_mode)
  (Variables|Movement|SetYaw (.Yaw (Math|Rotator|BreakRotator (Transformation|GetActorRotation))))
  (Variables|Default|SetSpawnLocation (Transformation|GetActorLocation))
  (bind _speed (Timeline|SpawnAnimation Play)
    (:Update
      (Transformation|SetActorLocationAndRotation (Math|Vector|Lerp(Vector) (Variables|Default|GetSpawnLocation) (+ (Variables|Default|GetSpawnLocation) "0, 0,60.000000") _speed) "0, 0, 0")
      (Transformation|SetActorRotation (Math|Rotator|Lerp(Rotator) "0, 0, 0" (Math|Rotator|MakeRotator 0.0 0.0 (+ (Variables|Movement|GetYaw) 1.44e+03)) _speed)))
    (:Finished
      (Variables|Movement|SetMoveEnabled true))))

(event EventTick
  (params (DeltaSeconds :type Float%20%28single-precision%29))
  (bind _returnvalue (Transformation|GetActorLocation))
  (bind _boosters (Variables|Default|GetBoosters))
  (bind _speed_multiplier (Variables|Movement|GetSpeed%20Multiplier))
  (bind _mobility_level (Variables|Mobility|GetMobility%20level))
  (bind _returnvalue_2 (Math|Conversions|ToFloat(Integer) _mobility_level))
  (bind _returnvalue_3 (* _returnvalue_2 1e+01))
  (bind _returnvalue_4 (+ _returnvalue_3 _speed_multiplier))
  ;[1 1 1] Movement
  (if (Variables|Default|GetIs%20Alive)
    (Variables|Default|SetDeltaSeconds DeltaSeconds)
    (CallFunction|HandleShootRequest)
    (if (>= (Variables|Movement|GetVertSpeed) 1.0)
      (Components|Activation|SetActive _boosters true false)
      (else
        (Components|Activation|SetActive _boosters false false)))
    (if (Math|Float|InRange(Float) (.y _returnvalue) -4.4e+02 4.4e+02)
      _
      (else
        (CallFunction|HandleOutOfMapException(YAxis))))
    (if (Math|Float|InRange(Float) (.z _returnvalue) -7.3e+02 7.3e+02)
      _
      (else
        (CallFunction|HandleOutOfMapException(ZAxis))))
    (Transformation|SetActorLocation (+ (Transformation|GetActorLocation) (Math|Vector|MakeVector 0.0 (* (Variables|Movement|GetHozSpeed) (Variables|Default|GetDeltaSeconds) _returnvalue_4) (* _returnvalue_4 (Variables|Default|GetDeltaSeconds) (Variables|Movement|GetVertSpeed)))) true false)
    (Transformation|SetActorRotation (Class|KismetMathLibrary|RInterptoConstant (Transformation|GetActorRotation) (Math|Rotator|MakeRotator 0.0 0.0 (+ (* (Variables|Movement|GetHozSpeed) 3.0) (Variables|Movement|GetYaw))) (Variables|Default|GetDeltaSeconds) 6e+01))
    (CallFunction|HandleEnemySpawn)
    (if (and (and (== (Variables|enemies|GetLiving%20Enemies) 0) (== (Variables|enemies|GetEnemies%20To%20Spawn) 0)) (not (Variables|Default|GetShop%20is%20on%20screen)))
      (CallFunction|SpawnShop))))

(event EventAddDamage
  (params (Damage :type Float%20%28single-precision%29))
  ;[1 1 1] Check Damage
  (CallFunction|+= (Variables|Default|GetDamage%20To%20Calculate) Damage)
  (if (> (Variables|Default|GetDamage%20To%20Calculate) 0.0)
    (Variables|Shield|SetTime%20From%20Last%20Damage 0.0)
    (if (< (Variables|Default|GetDamage%20To%20Calculate) (Variables|Shield|GetShield))
      ;;[1 1 1] Jeżeli obrażenia są mniejsze niż tarcza
      (Variables|Shield|SetShield (- (Variables|Shield|GetShield) (Variables|Default|GetDamage%20To%20Calculate)))
      (Variables|Default|SetDamage%20To%20Calculate 0.0)
      (CallFunction|CheckHPLevel :!label _label)
      (elif (== (Variables|Shield|GetShield) 0.0)
        ;;[1 1 1] Jeżeli tarcza jest równa zero
        (Variables|HP|SetHealth (- (Variables|HP|GetHealth) (Variables|Default|GetDamage%20To%20Calculate)))
        (Variables|Default|SetDamage%20To%20Calculate 0.0)
        (goto _label)
        (else
          ;;[1 1 1] Jeżeli tarcza jest większa niż zero ale mniejsza niż obrażenia
          (Variables|Default|SetDamage%20To%20Calculate (- (Variables|Default|GetDamage%20To%20Calculate) (Variables|Shield|GetShield)))
          (Variables|Shield|SetShield 0.0)
          (Audio|PlaySound2D "/Game/Assets/Sounds/Shield/Shield_down_Cue.Shield_down_Cue" 1.0 1.0 0.0 0 0)
          (CallFunction|AddDamage 0.0))))
    (else
      (CallFunction|HandleShieldRenew (Variables|Default|GetDeltaSeconds))
      (CallFunction|CheckHPLevel))))

(event Input|AxisEvents|InputAxisMoveUp
  (params (AxisValue :type Float%20%28single-precision%29))
  ;[1 1 1] Movement
  (bind _returndirectionspeed (CallFunction|Movement (Variables|Movement|GetHozSpeed) AxisValue))
  (Variables|Movement|SetHozSpeed _returndirectionspeed))

(event Input|AxisEvents|InputAxisMoveRight
  (params (AxisValue :type Float%20%28single-precision%29))
  (bind _returnvalue (* AxisValue -1.0))
  (bind _rocketeengineemitter (Variables|Default|GetRocketeEngineEmitter))
  ;[1 1 1] Movement
  (bind _returndirectionspeed (CallFunction|Movement (Variables|Movement|GetVertSpeed) _returnvalue))
  (Variables|Movement|SetVertSpeed _returndirectionspeed)
  (if (< _returnvalue 0.0)
    (Components|Activation|SetActive _rocketeengineemitter false false)
    (else
      (Components|Activation|SetActive _rocketeengineemitter true false))))

(event Input|KeyboardEvents|E
  (params (Key :type Key%20Structure :default "None"))
  ;[1 1 1] Rakiety
  (:Pressed
    (bind _outactors (Actor|GetAllActorsOfClass "/Game/Blueprint/enemies/BP_pirate.BP_pirate_C"))
    (if (<= (Utilities|Array|Length _outactors) 0)
      (Development|PrintString "brak przeciwników możliwych do namierzenia")
      (else
        (Game|SpawnActorfromClass "/Game/Blueprint/missiles/BP_Missile2.BP_Missile2_C" (Math|Transform|MakeTransform (Transformation|GetActorLocation) "0, 0, 0" "1,1,1") "Undefined" 0 5e+02 1 2e+01 0)))))

(fn ConstructionScript)

(fn Movement
  (params (Speed :type Float%20%28single-precision%29) (Direction :type Float%20%28single-precision%29))
  (return (Math|Interpolation|FInterpTo Speed (* (Variables|Movement|GetMovementSpeed) Direction) (Variables|Default|GetDeltaSeconds) 6.0)))

(fn HandleOutOfMapException
  (params (ActorLocation :type Vector) (HozSpeed :type Float%20%28single-precision%29) (VertSpeed :type Float%20%28single-precision%29) (Wrong%20Axis :type MovementAxises%20Enum :default "NewEnumerator0"))
  (bind _returnvalue (Utilities|Enum|Equal(Enum) Wrong%20Axis "NewEnumerator0"))
  (bind _returnvalue_2 (Math|Float|SelectFloat HozSpeed VertSpeed _returnvalue))
  (bind _returnvalue_3 (* -0.1 _returnvalue_2))
  (if (> (Math|Float|SelectFloat (.y ActorLocation) (.z ActorLocation) _returnvalue) 0.0)
    (if (>= _returnvalue_2 0.0)
      _
      (else
        (return HozSpeed VertSpeed)))
    (elif (<= _returnvalue_2 0.0)
      _
      (else
        (return HozSpeed VertSpeed))))
  (return (Math|Float|SelectFloat _returnvalue_3 HozSpeed _returnvalue) (Math|Float|SelectFloat VertSpeed _returnvalue_3 _returnvalue)))