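; Asteroid hazard that starts at a random Y at the top of the X=0 plane, with a random mesh, rotation and speed, and moves straight down on Tick.
; Overlapping the player deals random damage, notifies the player and plays its explosion component before delayed destruction.
; AddDamage drains HP, then spawns an explosion and BP_point and notifies the player on death.
; Reaching the bottom also triggers AddDamage each tick.
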(event EventBeginPlay
  (bind _returnvalue (Transformation|GetActorLocation))
  (bind _output_get (Variables|Default|SetCurrY (Math|Random|RandomFloatinRange -4.5e+02 4.5e+02)))
  (bind _output_get_2 (Variables|Default|SetcurrZ 9.2e+02))
  (Variables|Default|SetDepth 0.0)
  (Transformation|SetActorLocation (Math|Vector|MakeVector 0.0 _output_get _output_get_2) false true)
  (Variables|Default|SetmaxHP (Variables|Default|GetHP))
  (Variables|Default|SetTarget (Math|Vector|MakeVector (.x _returnvalue) (.y _returnvalue) -1e+03))
  (Variables|Default|SetInterp%20Speed (Math|Random|RandomFloatinRange (Variables|Default|GetInterp%20Speed) (Variables|Default|GetmaxSpeed)))
  (Components|StaticMesh|SetStaticMesh (Variables|Default|GetModel) (.OutItem (Utilities|Array|Random (Variables|Default|GetMeshes))))
  (Transformation|AddRelativeRotation (Variables|Default|GetModel) (Math|Random|RandomRotator true) false false))

(event Collision|EventActorBeginOverlap
  (params (OtherActor :type Actor%20Object%20Reference))
  (if (Variables|Default|GetisAlive)
    (bind _asbp_player (Utilities|Casting|CastToBP_Player OtherActor))
    (Class|DamageControll|AddDamage(Message) _asbp_player (Math|Random|RandomFloatinRange (Variables|Default|GetMinDmg) (Variables|Default|GetMaxDmg)))
    (Default|EnemyDestroyed _asbp_player "NewEnumerator1")
    (Components|Activation|SetActive (Variables|Default|GetExplosion) true false)
    (Rendering|SetVisibility (Variables|Default|GetModel) false false)
    (Variables|Default|SetisAlive false)
    (Utilities|FlowControl|Delay 0.5)
    (Components|Activation|SetActive (Variables|Default|GetExplosion) false false)
    (Utilities|FlowControl|Delay 2.0)
    (Actor|DestroyActor)))

(event EventTick
  (params (DeltaSeconds :type Float%20%28single-precision%29))
  (if (Variables|Default|GetisAlive)
    (Transformation|SetActorLocation (Math|Interpolation|VInterptoConstant (Transformation|GetActorLocation) (Variables|Default|GetTarget) (Utilities|Time|GetWorldDeltaSeconds) (Variables|Default|GetInterp%20Speed)) false false)
    (if (Math|Vector|Equal(Vector) (Transformation|GetActorLocation) (Variables|Default|GetTarget) 0.001)
      (CallFunction|AddDamage (Variables|Default|GetMaxDmg)))))

(event EventAddDamage
  (params (Damage :type Float%20%28single-precision%29))
  (bind _returnvalue (Transformation|GetActorTransform))
  ;[1 1 1] Sprawdza czy zyje
  (if (Variables|Default|GetisAlive)
    (Variables|Default|SetHP (- (Variables|Default|GetHP) Damage))
    (if (<= (Variables|Default|GetHP) 0.0) ; Czy nieżyje
      (Game|SpawnActorfromClass "/Game/Blueprint/asteroids/AsteroidExplosion.AsteroidExplosion_C" (Math|Transform|MakeTransform (.location _returnvalue) (.rotation _returnvalue) "1,1,1") "Undefined" 0 0.5 2.0 0)
      (Rendering|SetVisibility (Variables|Default|GetModel) false true)
      (bind _asbp_player (Utilities|Casting|CastToBP_Player (Game|Player|GetPlayerPawn 0)))
      (Default|EnemyDestroyed _asbp_player "NewEnumerator3")
      (Variables|Default|SetisAlive false)
      (Game|SpawnActorfromClass "/Game/Blueprint/enemies/BP_point.BP_point_C" (Transformation|GetActorTransform) "AlwaysSpawn" 0 "NewEnumerator0" 0)
      (Actor|DestroyActor))))

(fn ConstructionScript)